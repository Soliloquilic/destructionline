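; Game mode for local multiplayer that sets up four players, each with their own pawn, when play begins.
; SpawnPlayers creates three extra local players alongside the first, then spawns one 0_Base1 character per player at a shared elevated point.
; Each character receives its player index through PlayerInt and as an actor tag, then is possessed by the matching player controller.
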(event `self.ReceiveBeginPlay`
  (`self.Spawn Players`))

(fn `Spawn Players`
  (for _index (range 1 4)
    ;[1 1 1] Create Extra Players
    (`GameplayStatics.CreatePlayer` _index))
  ;[1 1 1] Spawn Character Actors and Possess
  (for _index_2 (range 4)
    (bind _returnvalue (`|SpawnActorFromClass` "/Game/Blueprints/Characters/0_Base1.0_Base1_C" (`KismetMathLibrary.MakeTransform` (0.0 0.0 2000.0)) "Undefined" "OverrideRootScale" null (struct) _index_2 null))
    (set `Actor.Tags` (`|MakeArray` (`KismetStringLibrary.Conv_StringToName` (`KismetStringLibrary.Conv_IntToString` _index_2))) _returnvalue)
    (`Controller.Possess` (`GameplayStatics.GetPlayerController` _index_2) _returnvalue)))

(fn `UserConstructionScript`)