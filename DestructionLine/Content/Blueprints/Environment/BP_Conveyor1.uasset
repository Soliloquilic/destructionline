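; BP_Conveyor1 is a conveyor that carries BP_MasterItem actors along its forward direction.
; Every tick it offsets each overlapping item without sweep, scaled by Speed and delta time.
; An item entering PipeCollision is dropped and its mesh is attached with snapped location and rotation, while unconnected logic would spawn and attach a BP_Pipe.
; The construction script counter-scales the Arrow against actor scale.
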(event `self.PipeCollision.OnComponentBeginOverlap`
  (params (OverlappedComponent :type "PrimitiveComponent Object Reference") (OtherActor :type "Actor Object Reference") (OtherComp :type "PrimitiveComponent Object Reference") (OtherBodyIndex :type Integer) (bFromSweep :type Boolean) (SweepResult :type "HitResult Structure (by ref)"))
  (bind _asbp_master_item (cast `/Game/Blueprints/Items/BP_MasterItem` OtherActor))
  (bind _output_get (set `self.ItemRef` _asbp_master_item))
  (`/Game/Blueprints/Items/BP_MasterItem.Drop` _output_get)
  (`SceneComponent.K2_AttachToComponent` (`/Game/Blueprints/Items/BP_MasterItem.StaticMesh` _output_get) null "None" "SnapToTarget" "SnapToTarget" "KeepWorld" true))

(event `self.ReceiveBeginPlay`)

(event `self.ReceiveTick`
  (params (DeltaSeconds :type "Float (single-precision)"))
  (for _array_element (`self.GetOverlappingActors` "/Game/Blueprints/Items/BP_MasterItem.BP_MasterItem_C")
    (`self.K2_AddActorWorldOffset` _array_element (* (`KismetMathLibrary.GetForwardVector` (`self.K2_GetActorRotation`)) (* DeltaSeconds (* (`self.Speed`) 100.0))) false false)))

(fn `UserConstructionScript`
  (`SceneComponent.SetRelativeScale3D` (`self.Arrow`) (/ (1.0 1.0 1.0) (`self.GetActorScale3D`))))