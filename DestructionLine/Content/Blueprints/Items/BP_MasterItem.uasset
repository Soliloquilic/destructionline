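; BP_MasterItem is an item actor that takes its mesh from ItemInfo and can be carried, dropped and binned for points.
; Interact toggles carrying on player 0's character, attaching to the "Grip" socket and notifying any active task, or running the Drop logic.
; Collision and physics switch between held and dropped states.
; Placing a non-weapon in a bin rebuilds PlayerInfo with 100 more round points.
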(event `Product Placed In Bin`
  (bind (_iteminfo_mesh _iteminfo_isweapon) (break `/Game/Blueprints/Items/Struct_ItemInfo` (`self.ItemInfo`)))
  (if (not _iteminfo_isweapon)
    (bind _as0_base_1 (cast `/Game/Blueprints/Characters/0_Base1` (`GameplayStatics.GetPlayerCharacter` 0)))
    (bind (_playerid _playername _rank _items_crafted _objectives_completed _bonus_tasks_completed _points_earned _players_knocked_out _players_hit_with_itemx _players_hit_with_itemy _players_hit_with_itemz _times_taunted _pointsround) (break `/Game/Data/Struct_PlayerInfo` (`/Game/Blueprints/Characters/0_Base1.PlayerInfo` _as0_base_1)))
    (set `/Game/Blueprints/Characters/0_Base1.PlayerInfo` (make `/Game/Data/Struct_PlayerInfo` _playerid _playername _rank _items_crafted _objectives_completed _bonus_tasks_completed _points_earned _players_knocked_out _players_hit_with_itemx _players_hit_with_itemy _players_hit_with_itemz _times_taunted (+ _pointsround 100)) _as0_base_1)))

(event `self.ReceiveBeginPlay`
  (bind _iteminfo_mesh (break `/Game/Blueprints/Items/Struct_ItemInfo` (`self.ItemInfo`)))
  (`StaticMeshComponent.SetStaticMesh` (`self.StaticMesh`) _iteminfo_mesh))

(event `Drop`
  (set `/Game/Blueprints/Characters/0_Base1.ActorIsAttached` false (stale `/Game/Blueprints/Objectives/Interface_Interact.Interact` _as0_base_1) :!label _label)
  (`self.K2_DetachFromActor` (stale `/Game/Blueprints/Objectives/Interface_Interact.Interact` _as0_base_1) "KeepWorld" "KeepWorld" "KeepWorld")
  (`PrimitiveComponent.SetSimulatePhysics` (`self.StaticMesh`) true)
  (`PrimitiveComponent.SetCollisionResponseToAllChannels` (`self.StaticMesh`) "ECR_Block")
  (bind _interactmessage (`/Game/Blueprints/Characters/0_Base1.InteractMessage` (stale `/Game/Blueprints/Objectives/Interface_Interact.Interact` _as0_base_1))
    (:`then`
      (`SceneComponent.ToggleVisibility` _interactmessage false))
    (:`else`)))

(event `/Game/Blueprints/Objectives/Interface_Interact.Interact`
  (bind _as0_base_1 (cast `/Game/Blueprints/Characters/0_Base1` (`GameplayStatics.GetPlayerCharacter` 0)))
  (set `/Game/Blueprints/Characters/0_Base1.AttachedActor` self _as0_base_1)
  (if (`/Game/Blueprints/Characters/0_Base1.ActorIsAttached` _as0_base_1)
    (goto _label)
    (else
      (set `/Game/Blueprints/Characters/0_Base1.ActorIsAttached` true _as0_base_1)
      (`PrimitiveComponent.SetCollisionResponseToAllChannels` (`self.StaticMesh`) "ECR_Overlap")
      (`KismetSystemLibrary.Delay` 0.01)
      (`self.K2_AttachToComponent` (`Character.Mesh` _as0_base_1) "Grip" "SnapToTarget" "SnapToTarget" "KeepWorld")
      (`PrimitiveComponent.SetSimulatePhysics` (`self.StaticMesh`) false)
      (`SceneComponent.ToggleVisibility` (`/Game/Blueprints/Characters/0_Base1.InteractMessage` _as0_base_1) false)
      (bind _taskref (`/Game/Blueprints/Characters/0_Base1.TaskRef` _as0_base_1)
        (:`then`
          (`/Game/Blueprints/Objectives/Tasks/BP_Task.CollectedItem` _taskref self))
        (:`else`)))))

(fn `UserConstructionScript`)